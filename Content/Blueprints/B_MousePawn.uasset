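; Mouse-driven pawn that lets the player click and drag actors in the YZ plane at X=0.
; On begin play it adds the IMC_Main input context and shows the cursor.
; IA_MouseClick traces under the cursor, prints the hit actor's name, stores it unless it is B_Background, and opens a Tick gate.
; While open, Tick moves that actor using the deprojected mouse position until click completion or cancellation clears it.
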(event Custom|CloseGate
  (bind _returnvalue (Game|GetPlayerController 0))
  (bind (_worldlocation _worlddirection) (Game|Player|ConvertMouseLocationToWorldSpace _returnvalue))
  (bind (_x _y _z) (Math|Vector|BreakVector _worlddirection))
  (bind (_x_2 _y_2 _z_2) (Math|Vector|BreakVector _worldlocation))
  (Utilities|FlowControl|Gate true) ; enters at Close
)

(event Input|EnhancedActionEvents|EnhancedInputActionIA_MouseClick
  (params (ActionValue :type Boolean) (ElapsedSeconds :type Float%20%28double-precision%29) (TriggeredSeconds :type Float%20%28double-precision%29) (InputAction :type Input%20Action%20Object%20Reference :default "/Game/Controller/Input/IA_MouseClick.IA_MouseClick"))
  (bind _returnvalue (Game|GetPlayerController 0))
  (bind _returnvalue_2 (Game|GetPlayerController 0))
  (bind _hitresult (Game|Player|GetHitResultUnderCursorbyChannel _returnvalue_2 "TraceTypeQuery1" true))
  (bind (_worldlocation _worlddirection) (Game|Player|ConvertMouseLocationToWorldSpace _returnvalue))
  (bind (_x _y _z) (Math|Vector|BreakVector _worlddirection))
  (bind (_x_2 _y_2 _z_2) (Math|Vector|BreakVector _worldlocation))
  (bind (_bblockinghit _binitialoverlap _time _distance _location _impactpoint _normal _impactnormal _physmat _hitactor) (Collision|BreakHitResult _hitresult))
  (:Triggered
    (if _bblockinghit
      (Development|PrintString (Utilities|GetDisplayName _hitactor))
      (Utilities|IsValid _hitactor
        (:Is%20Valid
          (Utilities|Casting|CastToB_Background _hitactor
            (:then
              (Variables|Default|SetHitActor 0))
            (:CastFailed
              (Variables|Default|SetHitActor _hitactor)
              (Utilities|FlowControl|Gate true) ; enters at Open
            ))))))
  (:Canceled
    (Variables|Default|SetHitActor 0 :!label _label)
    (Utilities|FlowControl|Gate true) ; enters at Close
  )
  (:Completed
    (goto _label)))

(event EventTick
  (params (DeltaSeconds :type Float%20%28single-precision%29))
  (bind _returnvalue (Game|GetPlayerController 0))
  (bind (_worldlocation _worlddirection) (Game|Player|ConvertMouseLocationToWorldSpace _returnvalue))
  (bind (_x _y _z) (Math|Vector|BreakVector _worlddirection))
  (bind (_x_2 _y_2 _z_2) (Math|Vector|BreakVector _worldlocation))
  (Utilities|FlowControl|Gate true
    (:Exit
      (Variables|Default|GetHitActor
        (:then
          (Transformation|SetActorLocation (Variables|Default|GetHitActor) (+ (Math|Vector|MakeVector 0.0 _y_2 _z_2) (* _worlddirection (Math|Vector|MakeVector 0.0 _y _z))) false false))
        (:else
          (CallFunction|CloseGate))))))

(event EventBeginPlay
  (bind _asplayer_controller (Utilities|Casting|CastToPlayerController (Pawn|GetController)))
  (Utilities|IsValid (PlayerController|LocalPlayerSubsystems|GetEnhancedInputLocalPlayerSubsystem _asplayer_controller)
    (:Is%20Valid
      (Input|AddMappingContext (PlayerController|LocalPlayerSubsystems|GetEnhancedInputLocalPlayerSubsystem _asplayer_controller) "/Game/Controller/Input/IMC_Main.IMC_Main" 0 "(bIgnoreAllPressedKeysUntilRelease=True,bForceImmediately=False,bNotifyUserSettings=False)")
      (Variables|/Script/Engine.PlayerController|SetbShowMouseCursor (Game|GetPlayerController 0) true))))

(fn ConstructionScript)