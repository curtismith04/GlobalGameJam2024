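; Main game state (GS_Main) for a zombie dress-up game, managing clothing spawns, scores and the ending camera cue.
; On BeginPlay it caches the zombie spline and target points, then fills a tag-to-data-asset map from clothing data tables.
; Spawning draws randomly from that map without replacement, reloading when empty, and picks the actor class by tag substring.
; Missed items teleport to a target point, while dispatchers broadcast scores and camera moves.
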(event Custom|ReloadArray
  (bind _outactors (Actor|GetAllActorsOfClass "/Script/Engine.TargetPoint"))
  (for _array_element _outactors
    (if (Actor|ActorHasTag _array_element "SpawnPoint")
      (Variables|Default|SetClothingSpawnPoint _array_element)
      (else
        (Variables|Default|SetMissedItemTarget _array_element))))
  (bind _outrownames (DataTable|GetDataTableRowNames (Variables|Default|GetClothingDatabase)))
  (for _array_element_2 _outrownames
    (bind _returnvalue (Utilities|GetDataTableRow "/Game/DataAssets/DT_ClothingOptions.DT_ClothingOptions" _array_element_2)
      (:then
        ;[1 1 1] Init the map
        (Utilities|Map|Add (Variables|Default|GetCurrentClothingMap) (.Tag (Utilities|Struct|BreakFClothingOptions _returnvalue)) (.PDA (Utilities|Struct|BreakFClothingOptions _returnvalue)))))))

(event EventBeginPlay
  (bind _returnvalue (Actor|GetActorOfClass "/Game/Blueprints/B_ZombieSpline.B_ZombieSpline_C"))
  (Variables|Default|SetZombieSpline _returnvalue)
  (bind _outactors (Actor|GetAllActorsOfClass "/Script/Engine.TargetPoint"))
  (for _array_element _outactors
    (if (Actor|ActorHasTag _array_element "SpawnPoint")
      (Variables|Default|SetClothingSpawnPoint _array_element)
      (else
        (Variables|Default|SetMissedItemTarget _array_element))))
  (bind _outrownames (DataTable|GetDataTableRowNames (Variables|Default|GetClothingDatabase)))
  (for _array_element_2 _outrownames
    (bind _returnvalue_2 (Utilities|GetDataTableRow "/Game/DataAssets/DT_ClothingOptions.DT_ClothingOptions" _array_element_2)
      (:then
        ;[1 1 1] Init the map
        (Utilities|Map|Add (Variables|Default|GetCurrentClothingMap) (.Tag (Utilities|Struct|BreakFClothingOptions _returnvalue_2)) (.PDA (Utilities|Struct|BreakFClothingOptions _returnvalue_2)))))))

(fn ConstructionScript)

(fn YeetCurrentClothing
  (params (ItemToYeet :type B%20Clothing%20Object%20Reference))
  (Transformation|SetActorLocation ItemToYeet (Transformation|GetActorLocation (Variables|Default|GetMissedItemTarget)) false false))

(fn UpdateClothingItem
  (bind _currentclothingmap (Variables|Default|GetCurrentClothingMap))
  (bind _currentclothingmap_2 (Variables|Default|GetCurrentClothingMap))
  (bind _returnvalue (Utilities|Map|Length _currentclothingmap_2))
  (if (> _returnvalue 0)
    (bind _keys (Utilities|Map|Keys _currentclothingmap))
    (bind _output_get (Variables|Default|SetSpawnedItemPDA (.Value (Utilities|Map|Find _currentclothingmap (Utilities|Array|Get(acopy) _keys (Math|Random|RandomIntegerinRange 0 (- _returnvalue 1)))))))
    (Variables|Default|SetSpawnedItemTexture (Variables|/Game/DataAssets/PDA_Items.PDA_Items_C|GetTexture _output_get))
    (Variables|Default|SetSpawnedItemTag (Utilities|Array|Get(acopy) _keys (Math|Random|RandomIntegerinRange 0 (- _returnvalue 1))))
    (Utilities|Map|Remove (Variables|Default|GetCurrentClothingMap) (Variables|Default|GetSpawnedItemTag))
    (Utilities|Map|Add (Variables|Default|GetUsedItems) (Variables|Default|GetSpawnedItemTag) (Variables|Default|GetSpawnedItemTexture))
    (Utilities|SwitchonItem "Chest" (Variables|Default|GetSpawnedItemTag)
      (:true
        (LocalVariables|SetSelctedIndex 0))
      (:false
        (Utilities|SwitchonItem "Feet" (Variables|Default|GetSpawnedItemTag)
          (:true
            (LocalVariables|SetSelctedIndex 1))
          (:false
            (Utilities|SwitchonItem "Hair" (Variables|Default|GetSpawnedItemTag)
              (:true
                (LocalVariables|SetSelctedIndex 2))
              (:false
                (Utilities|SwitchonItem "Prop" (Variables|Default|GetSpawnedItemTag)
                  (:true
                    (LocalVariables|SetSelctedIndex 3))
                  (:false
                    (Utilities|SwitchonItem "Legs" (Variables|Default|GetSpawnedItemTag)
                      (:true
                        (LocalVariables|SetSelctedIndex 4))
                      (:false
                        (Utilities|SwitchonItem "Face" (Variables|Default|GetSpawnedItemTag)
                          (:true
                            (LocalVariables|SetSelctedIndex 5)))))))))))))
    (return (Utilities|Select :Index (LocalVariables|GetSelctedIndex) :Option%200 "/Game/Blueprints/Clothing/B_Clothing_Chest.B_Clothing_Chest_C" :Option%201 "/Game/Blueprints/Clothing/B_Clothing_Feet.B_Clothing_Feet_C" :Option%202 "/Game/Blueprints/Clothing/B_Clothing_Hair.B_Clothing_Hair_C" :Option%203 "/Game/Blueprints/Clothing/B_Clothing_Item.B_Clothing_Item_C" :Option%204 "/Game/Blueprints/Clothing/B_Clothing_Legs.B_Clothing_Legs_C" :Option%205 "/Game/Blueprints/Clothing/B_Clothing_Face.B_Clothing_Face_C"))
    (else
      (Development|PrintString "ArrayEmpty")
      (CallFunction|ReloadArray))))

(fn SpawnClothingItem
  (bind _actor (CallFunction|UpdateClothingItem))
  (Game|SpawnActorfromClass _actor (Math|Transform|MakeTransform (Transformation|GetActorLocation (Variables|Default|GetClothingSpawnPoint)) (Math|Rotator|MakeRotator 0.0 (Math|Random|RandomFloatinRange 0.0 3.6e+02) 9e+01) "1.000000,1.000000,1.000000") "Undefined" "MultiplyWithRoot" 0 0))

(fn MoveCameratoEnding
  (Default|CallTellCameratoMove))

(fn UpdateScoreHUD
  (params (ClothingCurrentScore :type Float%20%28double-precision%29))
  (bind _output_get (Variables|Scoring|SetClothingCurrentScore ClothingCurrentScore))
  (Default|CallWhatIstheClothingScore _output_get))

(fn UpdateZmbieScoreHUD
  (params (NumZombDressed :type Integer))
  (bind _output_get (Variables|Scoring|SetNumZombDressed NumZombDressed))
  (Default|CallWhatIstheZombCount _output_get))