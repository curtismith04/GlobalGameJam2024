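; Zombie spawner actor that creates zombies at its location and slides them along the Y axis with timelines.
; SpawnAndMoveZombie, called by timer, registers each new zombie in GS_Main as current and on-screen, then eases it to the middle (Y = 0).
; MovetoEnd moves a given zombie toward an end position staggered by its index, lerping from its live location each update.
; Both timelines run at a slowed play rate set on BeginPlay.
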(event Custom|SpawnAndMoveZombie
  (bind _defaultsceneroot (Variables|Default|GetDefaultSceneRoot))
  (bind _as_gs_main (Variables|Default|GetAs%20GS%20Main))
  (bind _returnvalue (Transformation|GetWorldLocation _defaultsceneroot))
  (bind (_x _y _z) (Math|Vector|BreakVector _returnvalue))
  ;[1 0.1864 0.867] Called by timer
  (bind _returnvalue_2 (Game|SpawnActorfromClass "/Game/Blueprints/B_ZombieBase.B_ZombieBase_C" (Math|Transform|MakeTransform _returnvalue "0, 0, 0" "1.000000,1.000000,1.000000") "Undefined" "MultiplyWithRoot" 0 0))
  (bind _output_get (Variables|Default|SetFreshZombie _returnvalue_2))
  (Variables|/Game/Blueprints/GS_Main.GS_Main_C|SetCurrentZombieOnScreen _as_gs_main _output_get)
  (Utilities|Array|AddUnique (Variables|/Game/Blueprints/GS_Main.GS_Main_C|GetAllZombisOnScreen _as_gs_main) _output_get)
  (bind _newtrack_0 (Timeline|MoveToMiddleTL PlayFromStart)
    (:Update
      (Transformation|SetActorLocation (Variables|Default|GetFreshZombie) (Math|Vector|MakeVector _x (Math|Float|Lerp _y 0.0 _newtrack_0) _z) false false))))

(event EventBeginPlay
  (bind _asgs_main (Utilities|Casting|CastToGS_Main (Game|GetGameState)))
  (Variables|Default|SetAs%20GS%20Main _asgs_main)
  (Components|Timeline|SetPlayRate (Variables|Default|GetMoveToMiddleTL) 0.2))

(event EventMovetoEnd
  (params (Zombie :type B%20Zombie%20Base%20Object%20Reference) (Index :type Integer))
  (bind _returnvalue (Transformation|GetActorLocation Zombie))
  (bind (_x _y _z) (Math|Vector|BreakVector _returnvalue))
  (Variables|Default|SetStartingLoc _returnvalue)
  (bind _newtrack_0 (Timeline|Timeline PlayFromStart)
    (:Update
      (Transformation|SetActorLocation Zombie (Math|Vector|MakeVector _x (Math|Float|Lerp _y (|(Distance-((Int*0.100000)*Distance)) -1.5e+03 (Math|Conversions|ToFloat(Integer) Index)) _newtrack_0) _z) false false))))

(fn ConstructionScript)