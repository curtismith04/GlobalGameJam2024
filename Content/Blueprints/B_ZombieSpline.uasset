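; Spline actor that spawns zombie cable mounts (B_ZombieCableRoot) and slides them along its path.
; SpawnCableMount spawns a mount at the first spline point and tracks it in MountsInUse.
; MoveZombie picks start and end distances from each mount's closest spline position, restarting one shared timeline per mount.
; The timeline lerps distance along the spline to set the mount's location and rotation.
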(event Custom|MoveZombie
  (for _array_element (Variables|Default|GetMountsInUse)
    (Utilities|IsValid _array_element
      (:Is%20Valid
        (bind (_startlocation _endlocatin) (CallFunction|GetDistanceAlongSpline (Variables|/Game/Blueprints/B_ZombieCableRoot.B_ZombieCableRoot_C|GetCube _array_element)))
        (bind _float (Timeline|MoveZombieToMiddle PlayFromStart)
          (:Update
            (CallFunction|UpdateLocation _array_element _startlocation _endlocatin _float)))))))

(event EventBeginPlay
  (bind _asgs_main (Utilities|Casting|CastToGS_Main (Game|GetGameState)))
  (Variables|Default|SetAs%20GS%20Main _asgs_main))

(event Input|KeyboardEvents|DebugKeyO
  (params (Key :type Key%20Structure :default "None") (ActionValue :type Input%20Action%20Value%20Structure)))

(fn ConstructionScript)

(fn SpawnCableMount
  (bind _spline (Variables|Default|GetSpline))
  (bind _returnvalue (Spline|GetSplinePointAt _spline 0 "Local"))
  (bind _position (Utilities|Struct|BreakSplinePoint _returnvalue))
  (bind _returnvalue_2 (Game|SpawnActorfromClass "/Game/Blueprints/B_ZombieCableRoot.B_ZombieCableRoot_C" (Math|Transform|MakeTransform _position "0, 0, 0" "1.000000,1.000000,1.000000") "Undefined" "MultiplyWithRoot" 0 0))
  (Utilities|Array|AddUnique (Variables|Default|GetMountsInUse) _returnvalue_2)
  (return _returnvalue_2 _position))

(fn UpdateLocation
  (params (ActorToMove :type Actor%20Object%20Reference) (StartLocation :type Float%20%28double-precision%29) (EndLocation :type Float%20%28double-precision%29) (Alpha :type Float%20%28double-precision%29))
  (bind _returnvalue (Math|Float|Lerp StartLocation EndLocation Alpha))
  (bind _spline (Variables|Default|GetSpline))
  (Transformation|SetActorTransform ActorToMove (Math|Transform|MakeTransform (Spline|GetLocationatDistanceAlongSpline _spline _returnvalue "World") (Spline|GetRotationatDistanceAlongSpline _spline _returnvalue "Local") "1.000000,1.000000,1.000000")))

(fn GetDistanceAlongSpline
  (params (self2 :type Scene%20Component%20Object%20Reference))
  (bind _returnvalue (Transformation|GetWorldLocation self2))
  (bind _spline (Variables|Default|GetSpline))
  (bind _returnvalue_2 (Spline|FindLocationClosesttoWorldLocation _spline _returnvalue "World"))
  (bind _returnvalue_3 (Class|SplineComponent|GetDistanceAlongSplineatLocation _spline _returnvalue_2 "Local"))
  (bind _returnvalue_4 (> _returnvalue_3 0.2))
  (if _returnvalue_4
    _
    (else
      (bind _returnvalue_5 (CallFunction|GetEndLocation))))
  (return _returnvalue_3 (Math|Float|SelectFloat _returnvalue_5 0.5 _returnvalue_4)))

(fn GetEndLocation
  (bind _spline (Variables|Default|GetSpline))
  (return (Class|SplineComponent|GetDistanceAlongSplineatLocation _spline (.Position (Utilities|Struct|BreakSplinePoint (Spline|GetSplinePointAt _spline (Spline|GetNumberOfSplinePoints _spline) "Local"))) "Local")))