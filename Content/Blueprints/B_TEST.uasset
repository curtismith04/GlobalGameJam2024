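; Dress-up target actor with body-zone collision components (hair, face, chest, legs, hands, feet, prop) that accept dragged clothing.
; Each zone feeds a shared MountItem macro, which matches gameplay tags, mounts GS_Main's held clothing if the mouse is up, then plays its sound and raises the score.
; Release outside a zone calls YeetCurrentClothing.
; Feet overlap begin/end are wired in reverse, and dynamic material creation for UpdateImage is disconnected.
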(event OnComponentBeginOverlap(Face)
  (params (OverlappedComponent :type Primitive%20Component%20Object%20Reference) (OtherActor :type Actor%20Object%20Reference) (OtherComp :type Primitive%20Component%20Object%20Reference) (OtherBodyIndex :type Integer) (bFromSweep :type Boolean) (SweepResult :type Hit%20Result%20Structure%20%28by%20ref%29))
  ;[1 1 1] Face
  (Utilities|MountItem OtherActor (stale OnComponentEndOverlap(Face) OtherActor) "Face"))

(event OnComponentBeginOverlap(Hair)
  (params (OverlappedComponent :type Primitive%20Component%20Object%20Reference) (OtherActor :type Actor%20Object%20Reference) (OtherComp :type Primitive%20Component%20Object%20Reference) (OtherBodyIndex :type Integer) (bFromSweep :type Boolean) (SweepResult :type Hit%20Result%20Structure%20%28by%20ref%29))
  ;[1 1 1] Hair
  (Utilities|MountItem OtherActor (stale OnComponentEndOverlap(Hair) OtherActor) "Hair"))

(event OnReleased(Hair)
  (params (TouchedComponent :type Primitive%20Component%20Object%20Reference) (ButtonReleased :type Key%20Structure :default "None"))
  ;[1 1 1] Hair
  (Utilities|MountItem (stale OnComponentBeginOverlap(Hair) OtherActor) (stale OnComponentEndOverlap(Hair) OtherActor) "Hair") ; enters at OnRelease
)

(event OnComponentEndOverlap(Hair)
  (params (OverlappedComponent :type Primitive%20Component%20Object%20Reference) (OtherActor :type Actor%20Object%20Reference) (OtherComp :type Primitive%20Component%20Object%20Reference) (OtherBodyIndex :type Integer))
  ;[1 1 1] Hair
  (Utilities|MountItem (stale OnComponentBeginOverlap(Hair) OtherActor) OtherActor "Hair") ; enters at EndOverlap
)

(event OnComponentEndOverlap(Chest)
  (params (OverlappedComponent :type Primitive%20Component%20Object%20Reference) (OtherActor :type Actor%20Object%20Reference) (OtherComp :type Primitive%20Component%20Object%20Reference) (OtherBodyIndex :type Integer))
  ;[1 1 1] Chest
  (Utilities|MountItem (stale OnComponentBeginOverlap(Chest) OtherActor) OtherActor "Chest") ; enters at EndOverlap
)

(event OnReleased(Chest)
  (params (TouchedComponent :type Primitive%20Component%20Object%20Reference) (ButtonReleased :type Key%20Structure :default "None"))
  ;[1 1 1] Chest
  (Utilities|MountItem (stale OnComponentBeginOverlap(Chest) OtherActor) (stale OnComponentEndOverlap(Chest) OtherActor) "Chest") ; enters at OnRelease
)

(event OnComponentEndOverlap(Legs)
  (params (OverlappedComponent :type Primitive%20Component%20Object%20Reference) (OtherActor :type Actor%20Object%20Reference) (OtherComp :type Primitive%20Component%20Object%20Reference) (OtherBodyIndex :type Integer))
  ;[1 1 1] legs
  (Utilities|MountItem (stale OnComponentBeginOverlap(Legs) OtherActor) OtherActor "Legs") ; enters at EndOverlap
)

(event OnReleased(Legs)
  (params (TouchedComponent :type Primitive%20Component%20Object%20Reference) (ButtonReleased :type Key%20Structure :default "None"))
  ;[1 1 1] legs
  (Utilities|MountItem (stale OnComponentBeginOverlap(Legs) OtherActor) (stale OnComponentEndOverlap(Legs) OtherActor) "Legs") ; enters at OnRelease
)

(event OnComponentEndOverlap(Prop)
  (params (OverlappedComponent :type Primitive%20Component%20Object%20Reference) (OtherActor :type Actor%20Object%20Reference) (OtherComp :type Primitive%20Component%20Object%20Reference) (OtherBodyIndex :type Integer))
  ;[1 1 1] Props
  (Utilities|MountItem (stale OnComponentBeginOverlap(Prop) OtherActor) OtherActor "Hand") ; enters at EndOverlap
)

(event OnReleased(Prop)
  (params (TouchedComponent :type Primitive%20Component%20Object%20Reference) (ButtonReleased :type Key%20Structure :default "None"))
  ;[1 1 1] Props
  (Utilities|MountItem (stale OnComponentBeginOverlap(Prop) OtherActor) (stale OnComponentEndOverlap(Prop) OtherActor) "Hand") ; enters at OnRelease
)

(event OnComponentEndOverlap(Feet)
  (params (OverlappedComponent :type Primitive%20Component%20Object%20Reference) (OtherActor :type Actor%20Object%20Reference) (OtherComp :type Primitive%20Component%20Object%20Reference) (OtherBodyIndex :type Integer))
  ;[1 1 1] Feet
  (Utilities|MountItem OtherActor (stale OnComponentBeginOverlap(Feet) OtherActor) "Feet"))

(event OnReleased(Feet)
  (params (TouchedComponent :type Primitive%20Component%20Object%20Reference) (ButtonReleased :type Key%20Structure :default "None"))
  ;[1 1 1] Feet
  (Utilities|MountItem (stale OnComponentEndOverlap(Feet) OtherActor) (stale OnComponentBeginOverlap(Feet) OtherActor) "Feet") ; enters at OnRelease
)

(event OnComponentBeginOverlap(Chest)
  (params (OverlappedComponent :type Primitive%20Component%20Object%20Reference) (OtherActor :type Actor%20Object%20Reference) (OtherComp :type Primitive%20Component%20Object%20Reference) (OtherBodyIndex :type Integer) (bFromSweep :type Boolean) (SweepResult :type Hit%20Result%20Structure%20%28by%20ref%29))
  ;[1 1 1] Chest
  (Utilities|MountItem OtherActor (stale OnComponentEndOverlap(Chest) OtherActor) "Chest"))

(event OnComponentEndOverlap(Hands)
  (params (OverlappedComponent :type Primitive%20Component%20Object%20Reference) (OtherActor :type Actor%20Object%20Reference) (OtherComp :type Primitive%20Component%20Object%20Reference) (OtherBodyIndex :type Integer))
  (Utilities|MountItem (stale OnComponentBeginOverlap(Hands) OtherActor) OtherActor "Hand") ; enters at EndOverlap
)

(event OnBeginCursorOver(Chest)
  (params (TouchedComponent :type Primitive%20Component%20Object%20Reference)))

(event OnComponentBeginOverlap(Legs)
  (params (OverlappedComponent :type Primitive%20Component%20Object%20Reference) (OtherActor :type Actor%20Object%20Reference) (OtherComp :type Primitive%20Component%20Object%20Reference) (OtherBodyIndex :type Integer) (bFromSweep :type Boolean) (SweepResult :type Hit%20Result%20Structure%20%28by%20ref%29))
  ;[1 1 1] legs
  (Utilities|MountItem OtherActor (stale OnComponentEndOverlap(Legs) OtherActor) "Legs"))

(event OnComponentBeginOverlap(Prop)
  (params (OverlappedComponent :type Primitive%20Component%20Object%20Reference) (OtherActor :type Actor%20Object%20Reference) (OtherComp :type Primitive%20Component%20Object%20Reference) (OtherBodyIndex :type Integer) (bFromSweep :type Boolean) (SweepResult :type Hit%20Result%20Structure%20%28by%20ref%29))
  ;[1 1 1] Props
  (Utilities|MountItem OtherActor (stale OnComponentEndOverlap(Prop) OtherActor) "Hand"))

(event OnComponentBeginOverlap(Feet)
  (params (OverlappedComponent :type Primitive%20Component%20Object%20Reference) (OtherActor :type Actor%20Object%20Reference) (OtherComp :type Primitive%20Component%20Object%20Reference) (OtherBodyIndex :type Integer) (bFromSweep :type Boolean) (SweepResult :type Hit%20Result%20Structure%20%28by%20ref%29))
  ;[1 1 1] Feet
  (Utilities|MountItem (stale OnComponentEndOverlap(Feet) OtherActor) OtherActor "Feet") ; enters at EndOverlap
)

(event OnComponentBeginOverlap(Hands)
  (params (OverlappedComponent :type Primitive%20Component%20Object%20Reference) (OtherActor :type Actor%20Object%20Reference) (OtherComp :type Primitive%20Component%20Object%20Reference) (OtherBodyIndex :type Integer) (bFromSweep :type Boolean) (SweepResult :type Hit%20Result%20Structure%20%28by%20ref%29))
  (Utilities|MountItem OtherActor (stale OnComponentEndOverlap(Hands) OtherActor) "Hand"))

(event OnComponentEndOverlap(Face)
  (params (OverlappedComponent :type Primitive%20Component%20Object%20Reference) (OtherActor :type Actor%20Object%20Reference) (OtherComp :type Primitive%20Component%20Object%20Reference) (OtherBodyIndex :type Integer))
  ;[1 1 1] Face
  (Utilities|MountItem (stale OnComponentBeginOverlap(Face) OtherActor) OtherActor "Face") ; enters at EndOverlap
)

(event OnReleased(Face)
  (params (TouchedComponent :type Primitive%20Component%20Object%20Reference) (ButtonReleased :type Key%20Structure :default "None"))
  ;[1 1 1] Face
  (Utilities|MountItem (stale OnComponentBeginOverlap(Face) OtherActor) (stale OnComponentEndOverlap(Face) OtherActor) "Face") ; enters at OnRelease
)

(event OnReleased(Hands)
  (params (TouchedComponent :type Primitive%20Component%20Object%20Reference) (ButtonReleased :type Key%20Structure :default "None"))
  (Utilities|MountItem (stale OnComponentBeginOverlap(Hands) OtherActor) (stale OnComponentEndOverlap(Hands) OtherActor) "Hand") ; enters at OnRelease
)

(event Custom|UpdateImage
  (params (Texture :type Texture%20Object%20Reference))
  (Rendering|Material|SetTextureParameterValue (Variables|Default|GetDynamicmaterial) "Image" Texture))

(event Custom|AddItem
  (params (Clothing :type E_Clothing%20Enum :default "NewEnumerator0"))
  (switch Utilities|FlowControl|Switch|SwitchonE_Clothing Clothing
    (:NewEnumerator0
      (if (not (Variables|Default|GetbIsHairAttched))
        (Variables|Default|SetbIsHairAttched true)))
    (:NewEnumerator1
      (if (not (Variables|Default|GetbIsFaceAttached))
        (Variables|Default|SetbIsFaceAttached true)))
    (:NewEnumerator2
      (if (not (Variables|Default|GetbIsChestAttached))
        (Variables|Default|SetbIsChestAttached true)))
    (:NewEnumerator3
      (if (not (Variables|Default|GetbIsLegsAttached))
        (Variables|Default|SetbIsLegsAttached true)))
    (:NewEnumerator4
      (if (not (Variables|Default|GetbIsHandsAttached))
        (Variables|Default|SetbIsHandsAttached true)))
    (:NewEnumerator5
      (if (not (Variables|Default|GetbIsFeetAttached))
        (Variables|Default|SetbIsFeetAttached true)))))

(event Input|EnhancedActionEvents|EnhancedInputActionIA_MouseClick
  (params (ActionValue :type Boolean) (ElapsedSeconds :type Float%20%28double-precision%29) (TriggeredSeconds :type Float%20%28double-precision%29) (InputAction :type Input%20Action%20Object%20Reference :default "/Game/Controller/Input/IA_MouseClick.IA_MouseClick"))
  (:Triggered
    (Variables|Default|SetbIsMousebuttonDown true :!label _label))
  (:Ongoing
    (goto _label))
  (:Canceled
    (Variables|Default|SetbIsMousebuttonDown false :!label _label_2))
  (:Completed
    (goto _label_2)))

(event EventBeginPlay
  (bind _asgs_main (Utilities|Casting|CastToGS_Main (Game|GetGameState)))
  (Variables|Default|SetAs%20GS%20Main _asgs_main)
  (bind _asb_mouse_pawn (Utilities|Casting|CastToB_MousePawn (Game|Player|GetPlayerPawn 0)))
  (Variables|Default|SetAs%20B%20Mouse%20Pawn _asb_mouse_pawn))

(fn ConstructionScript)